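; Base enemy Blueprint, named as an old version, that detects and damages the VR player by line of sight.
; While the game instance's Looking flag is set, Tick fires a debug-drawn fan of visibility traces from its Camera in two pitch rows.
; Any VRPawn hit subtracts player HP every tick and briefly shows a component on the pawn.
; The Spotted function is an empty stub.
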(event EventTick
  (params (DeltaSeconds :type Float%20%28single-precision%29))
  (bind _vrpawnref (Variables|Default|GetVRPawnRef))
  (bind _camera (Variables|Default|GetCamera))
  (bind _camera_2 (Variables|Default|GetCamera))
  (bind _camera_3 (Variables|Default|GetCamera))
  (bind _camera_4 (Variables|Default|GetCamera))
  (bind _camera_5 (Variables|Default|GetCamera))
  (bind _camera_6 (Variables|Default|GetCamera))
  (bind _camera_7 (Variables|Default|GetCamera))
  (bind _camera_8 (Variables|Default|GetCamera))
  (bind _camera_9 (Variables|Default|GetCamera))
  (bind _camera_10 (Variables|Default|GetCamera))
  (bind _camera_11 (Variables|Default|GetCamera))
  (bind _camera_12 (Variables|Default|GetCamera))
  (bind _camera_13 (Variables|Default|GetCamera))
  (bind _camera_14 (Variables|Default|GetCamera))
  (bind _camera_15 (Variables|Default|GetCamera))
  (bind _camera_16 (Variables|Default|GetCamera))
  (bind _camera_17 (Variables|Default|GetCamera))
  (bind _camera_18 (Variables|Default|GetCamera))
  (bind _returnvalue (Transformation|GetWorldLocation _camera_10))
  (bind _returnvalue_2 (Transformation|GetWorldLocation _camera_9))
  (bind _returnvalue_3 (Transformation|GetWorldRotation _camera_9))
  (bind _returnvalue_4 (Transformation|GetWorldLocation _camera_11))
  (bind _returnvalue_5 (Transformation|GetWorldRotation _camera_11))
  (bind _returnvalue_6 (Transformation|GetWorldLocation _camera_12))
  (bind _returnvalue_7 (Transformation|GetWorldRotation _camera_12))
  (bind _returnvalue_8 (Transformation|GetWorldRotation _camera_10))
  (bind _returnvalue_9 (Transformation|GetWorldLocation _camera_13))
  (bind _returnvalue_10 (Transformation|GetWorldRotation _camera_13))
  (bind _returnvalue_11 (Transformation|GetWorldLocation _camera_14))
  (bind _returnvalue_12 (Transformation|GetWorldRotation _camera_14))
  (bind _returnvalue_13 (Transformation|GetWorldLocation _camera_15))
  (bind _returnvalue_14 (Transformation|GetWorldRotation _camera_15))
  (bind _returnvalue_15 (Transformation|GetWorldLocation _camera_16))
  (bind _returnvalue_16 (Transformation|GetWorldRotation _camera_16))
  (bind _returnvalue_17 (Transformation|GetWorldLocation _camera_17))
  (bind _returnvalue_18 (Transformation|GetWorldRotation _camera_17))
  (bind _returnvalue_19 (Transformation|GetWorldLocation _camera_18))
  (bind _returnvalue_20 (Transformation|GetWorldLocation _camera))
  (bind _returnvalue_21 (Transformation|GetWorldRotation _camera))
  (bind _returnvalue_22 (Transformation|GetWorldLocation _camera_2))
  (bind _returnvalue_23 (Transformation|GetWorldRotation _camera_2))
  (bind _returnvalue_24 (Transformation|GetWorldLocation _camera_3))
  (bind _returnvalue_25 (Transformation|GetWorldRotation _camera_3))
  (bind _returnvalue_26 (Transformation|GetWorldLocation _camera_4))
  (bind _returnvalue_27 (Transformation|GetWorldRotation _camera_4))
  (bind _returnvalue_28 (Transformation|GetWorldLocation _camera_5))
  (bind _returnvalue_29 (Transformation|GetWorldRotation _camera_5))
  (bind _returnvalue_30 (Transformation|GetWorldLocation _camera_6))
  (bind _returnvalue_31 (Transformation|GetWorldRotation _camera_6))
  (bind _returnvalue_32 (Transformation|GetWorldLocation _camera_7))
  (bind _returnvalue_33 (Transformation|GetWorldRotation _camera_7))
  (bind _returnvalue_34 (Transformation|GetWorldLocation _camera_8))
  (bind _returnvalue_35 (Transformation|GetWorldRotation _camera_8))
  (bind __ (Variables|/Game/VRTemplate/Blueprints/VRPawn.VRPawn_C|Get! _vrpawnref))
  (if (Variables|/Game/Blueprints/HOP_GI.HOP_GI_C|GetLooking (.AsHOP%20GI (Utilities|Casting|CastToHOP_GI (Game|GetGameInstance))))
    (bind _outhit (Collision|LineTraceByChannel _returnvalue_19 (+ _returnvalue_19 (* (Math|Vector|GetForwardVector (Transformation|GetWorldRotation _camera_18)) 1.5e+03)) "TraceTypeQuery1" false 0 "ForOneFrame"))
    (bind _outhit_2 (Collision|LineTraceByChannel _returnvalue_20 (+ _returnvalue_20 (* (Math|Vector|GetForwardVector (Math|Rotator|MakeRotator (.roll _returnvalue_21) (.pitch _returnvalue_21) (+ (.yaw _returnvalue_21) 5.0))) 1.5e+03)) "TraceTypeQuery1" false 0 "ForOneFrame"))
    (bind _outhit_3 (Collision|LineTraceByChannel _returnvalue_22 (+ _returnvalue_22 (* (Math|Vector|GetForwardVector (Math|Rotator|MakeRotator (.roll _returnvalue_23) (.pitch _returnvalue_23) (+ (.yaw _returnvalue_23) -5.0))) 1.5e+03)) "TraceTypeQuery1" false 0 "ForOneFrame"))
    (bind _outhit_4 (Collision|LineTraceByChannel _returnvalue_24 (+ _returnvalue_24 (* (Math|Vector|GetForwardVector (Math|Rotator|MakeRotator (.roll _returnvalue_25) (.pitch _returnvalue_25) (+ (.yaw _returnvalue_25) 1e+01))) 1.5e+03)) "TraceTypeQuery1" false 0 "ForOneFrame"))
    (bind _outhit_5 (Collision|LineTraceByChannel _returnvalue_26 (+ _returnvalue_26 (* (Math|Vector|GetForwardVector (Math|Rotator|MakeRotator (.roll _returnvalue_27) (.pitch _returnvalue_27) (+ (.yaw _returnvalue_27) -1e+01))) 1.5e+03)) "TraceTypeQuery1" false 0 "ForOneFrame"))
    (bind _outhit_6 (Collision|LineTraceByChannel _returnvalue_28 (+ _returnvalue_28 (* (Math|Vector|GetForwardVector (Math|Rotator|MakeRotator (.roll _returnvalue_29) (.pitch _returnvalue_29) (+ (.yaw _returnvalue_29) 15.0))) 1.5e+03)) "TraceTypeQuery1" false 0 "ForOneFrame"))
    (bind _outhit_7 (Collision|LineTraceByChannel _returnvalue_30 (+ _returnvalue_30 (* (Math|Vector|GetForwardVector (Math|Rotator|MakeRotator (.roll _returnvalue_31) (.pitch _returnvalue_31) (+ (.yaw _returnvalue_31) -15.0))) 1.5e+03)) "TraceTypeQuery1" false 0 "ForOneFrame"))
    (bind _outhit_8 (Collision|LineTraceByChannel _returnvalue_32 (+ _returnvalue_32 (* (Math|Vector|GetForwardVector (Math|Rotator|MakeRotator (.roll _returnvalue_33) (.pitch _returnvalue_33) (+ (.yaw _returnvalue_33) 2e+01))) 1.5e+03)) "TraceTypeQuery1" false 0 "ForOneFrame"))
    (bind _outhit_9 (Collision|LineTraceByChannel _returnvalue_34 (+ _returnvalue_34 (* (Math|Vector|GetForwardVector (Math|Rotator|MakeRotator (.roll _returnvalue_35) (.pitch _returnvalue_35) (+ (.yaw _returnvalue_35) -2e+01))) 1.5e+03)) "TraceTypeQuery1" false 0 "ForOneFrame"))
    (bind _outhit_10 (Collision|LineTraceByChannel _returnvalue_4 (+ _returnvalue_4 (* (Math|Vector|GetForwardVector (Math|Rotator|MakeRotator (.roll _returnvalue_5) (+ (.pitch _returnvalue_5) -5.0) (+ (.yaw _returnvalue_5) 5.0))) 1.5e+03)) "TraceTypeQuery1" false 0 "ForOneFrame"))
    (bind _outhit_11 (Collision|LineTraceByChannel _returnvalue_2 (+ _returnvalue_2 (* (Math|Vector|GetForwardVector (Math|Rotator|MakeRotator (.roll _returnvalue_3) (+ (.pitch _returnvalue_3) -5.0) (+ (.yaw _returnvalue_3) 5.0))) 1.5e+03)) "TraceTypeQuery1" false 0 "ForOneFrame"))
    (bind _outhit_12 (Collision|LineTraceByChannel _returnvalue_6 (+ _returnvalue_6 (* (Math|Vector|GetForwardVector (Math|Rotator|MakeRotator (.roll _returnvalue_7) (+ (.pitch _returnvalue_7) -5.0) (+ (.yaw _returnvalue_7) -5.0))) 1.5e+03)) "TraceTypeQuery1" false 0 "ForOneFrame"))
    (bind _outhit_13 (Collision|LineTraceByChannel _returnvalue_9 (+ _returnvalue_9 (* (Math|Vector|GetForwardVector (Math|Rotator|MakeRotator (.roll _returnvalue_10) (+ (.pitch _returnvalue_10) -5.0) (+ (.yaw _returnvalue_10) 1e+01))) 1.5e+03)) "TraceTypeQuery1" false 0 "ForOneFrame"))
    (bind _outhit_14 (Collision|LineTraceByChannel _returnvalue_11 (+ _returnvalue_11 (* (Math|Vector|GetForwardVector (Math|Rotator|MakeRotator (.roll _returnvalue_12) (+ (.pitch _returnvalue_12) -5.0) (+ (.yaw _returnvalue_12) -1e+01))) 1.5e+03)) "TraceTypeQuery1" false 0 "ForOneFrame"))
    (bind _outhit_15 (Collision|LineTraceByChannel _returnvalue_13 (+ _returnvalue_13 (* (Math|Vector|GetForwardVector (Math|Rotator|MakeRotator (.roll _returnvalue_14) (+ (.pitch _returnvalue_14) -5.0) (+ (.yaw _returnvalue_14) 15.0))) 1.5e+03)) "TraceTypeQuery1" false 0 "ForOneFrame"))
    (bind _outhit_16 (Collision|LineTraceByChannel _returnvalue_15 (+ _returnvalue_15 (* (Math|Vector|GetForwardVector (Math|Rotator|MakeRotator (.roll _returnvalue_16) (+ (.pitch _returnvalue_16) -5.0) (+ (.yaw _returnvalue_16) -15.0))) 1.5e+03)) "TraceTypeQuery1" false 0 "ForOneFrame"))
    (bind _outhit_17 (Collision|LineTraceByChannel _returnvalue_17 (+ _returnvalue_17 (* (Math|Vector|GetForwardVector (Math|Rotator|MakeRotator (.roll _returnvalue_18) (+ (.pitch _returnvalue_18) -5.0) (+ (.yaw _returnvalue_18) 2e+01))) 1.5e+03)) "TraceTypeQuery1" false 0 "ForOneFrame"))
    (bind _outhit_18 (Collision|LineTraceByChannel _returnvalue (+ _returnvalue (* (Math|Vector|GetForwardVector (Math|Rotator|MakeRotator (.roll _returnvalue_8) (+ (.pitch _returnvalue_8) -5.0) (+ (.yaw _returnvalue_8) -2e+01))) 1.5e+03)) "TraceTypeQuery1" false 0 "ForOneFrame"))
    (if (Math|Boolean|ORBoolean (.bSuccess (Utilities|Casting|CastToVRPawn (.HitActor (Collision|BreakHitResult _outhit)))) (.bSuccess (Utilities|Casting|CastToVRPawn (.HitActor (Collision|BreakHitResult _outhit_2)))) (.bSuccess (Utilities|Casting|CastToVRPawn (.HitActor (Collision|BreakHitResult _outhit_3)))) (.bSuccess (Utilities|Casting|CastToVRPawn (.HitActor (Collision|BreakHitResult _outhit_4)))) (.bSuccess (Utilities|Casting|CastToVRPawn (.HitActor (Collision|BreakHitResult _outhit_5)))) (.bSuccess (Utilities|Casting|CastToVRPawn (.HitActor (Collision|BreakHitResult _outhit_6)))) (.bSuccess (Utilities|Casting|CastToVRPawn (.HitActor (Collision|BreakHitResult _outhit_7)))) (.bSuccess (Utilities|Casting|CastToVRPawn (.HitActor (Collision|BreakHitResult _outhit_8)))) (.bSuccess (Utilities|Casting|CastToVRPawn (.HitActor (Collision|BreakHitResult _outhit_9)))) (.bSuccess (Utilities|Casting|CastToVRPawn (.HitActor (Collision|BreakHitResult _outhit_10)))) (.bSuccess (Utilities|Casting|CastToVRPawn (.HitActor (Collision|BreakHitResult _outhit_11)))) (.bSuccess (Utilities|Casting|CastToVRPawn (.HitActor (Collision|BreakHitResult _outhit_12)))) (.bSuccess (Utilities|Casting|CastToVRPawn (.HitActor (Collision|BreakHitResult _outhit_13)))) (.bSuccess (Utilities|Casting|CastToVRPawn (.HitActor (Collision|BreakHitResult _outhit_14)))) (.bSuccess (Utilities|Casting|CastToVRPawn (.HitActor (Collision|BreakHitResult _outhit_15)))) (.bSuccess (Utilities|Casting|CastToVRPawn (.HitActor (Collision|BreakHitResult _outhit_16)))) (.bSuccess (Utilities|Casting|CastToVRPawn (.HitActor (Collision|BreakHitResult _outhit_17)))) (.bSuccess (Utilities|Casting|CastToVRPawn (.HitActor (Collision|BreakHitResult _outhit_18)))))
      (Variables|/Game/VRTemplate/Blueprints/VRPawn.VRPawn_C|SetPlayerHP _vrpawnref (- (Variables|/Game/VRTemplate/Blueprints/VRPawn.VRPawn_C|GetPlayerHP _vrpawnref) 3))
      (Rendering|SetVisibility __ true false)
      (Utilities|FlowControl|Delay 1.0)
      (Rendering|SetVisibility __ false false))))

(event EventBeginPlay
  (bind _outactors (Actor|GetAllActorsOfClass "/Game/VRTemplate/Blueprints/VRPawn.VRPawn_C"))
  (Variables|Default|SetVRPawnRef (Utilities|Array|Get(acopy) _outactors)))

(fn ConstructionScript)

(fn Spotted)