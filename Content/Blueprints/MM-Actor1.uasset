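; VR pawn that relays head and hand transforms, apparently for multiplayer, and lets the player click widgets with either motion controller.
; Tick sends camera and controller world transforms, behind short Delays, through paired relay events (camera's suffixed S and M) that re-apply them.
; BeginPlay enables replication and adds input mappings, whose trigger actions press and release each hand's widget pointer.
; Each tick also rebuilds spline mesh lasers toward hovered widgets.
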(event Custom|CamReplicateM
  (params (New%20Rotation%20Y%20%28Pitch%29 :type Float%20%28single-precision%29) (New%20Rotation%20Z%20%28Yaw%29 :type Float%20%28single-precision%29) (New%20Rotation%20X%20%28Roll%29 :type Float%20%28single-precision%29))
  (Transformation|SetWorldRotation (Variables|Default|GetCamera) (Math|Rotator|MakeRotator New%20Rotation%20X%20%28Roll%29 New%20Rotation%20Y%20%28Pitch%29 New%20Rotation%20Z%20%28Yaw%29) false false))

(event Custom|RightLo
  (params (New%20Location%20Y :type Float%20%28double-precision%29) (New%20Location%20X :type Float%20%28double-precision%29) (New%20Location%20Z :type Float%20%28double-precision%29))
  (CallFunction|RightControllerLoc New%20Location%20Y New%20Location%20X New%20Location%20Z))

(event Custom|RightControllerLoc
  (params (New%20Location%20Y :type Float%20%28double-precision%29) (New%20Location%20X :type Float%20%28double-precision%29) (New%20Location%20Z :type Float%20%28double-precision%29))
  (Transformation|SetWorldLocation (Variables|Default|GetMotionControllerRight) (Math|Vector|MakeVector New%20Location%20X New%20Location%20Y New%20Location%20Z) false false))

(event Custom|CamReplicateS
  (params (New%20Rotation%20Y%20%28Pitch%29 :type Float%20%28single-precision%29) (New%20Rotation%20X%20%28Roll%29 :type Float%20%28single-precision%29) (New%20Rotation%20Z%20%28Yaw%29 :type Float%20%28single-precision%29))
  (CallFunction|CamReplicateM New%20Rotation%20Y%20%28Pitch%29 New%20Rotation%20Z%20%28Yaw%29 New%20Rotation%20X%20%28Roll%29))

(event Custom|CamMoveS
  (params (New%20Location%20Y :type Float%20%28double-precision%29) (New%20Location%20X :type Float%20%28double-precision%29) (New%20Location%20Z :type Float%20%28double-precision%29))
  (CallFunction|CamMoveM New%20Location%20Y New%20Location%20X New%20Location%20Z))

(event Custom|LeftRo
  (params (New%20Rotation%20Y%20%28Pitch%29 :type Float%20%28single-precision%29) (New%20Rotation%20X%20%28Roll%29 :type Float%20%28single-precision%29) (New%20Rotation%20Z%20%28Yaw%29 :type Float%20%28single-precision%29))
  (CallFunction|LeftControllerRot New%20Rotation%20Y%20%28Pitch%29 New%20Rotation%20Z%20%28Yaw%29 New%20Rotation%20X%20%28Roll%29))

(event Custom|Left%20ControllerRot
  (params (New%20Rotation%20Y%20%28Pitch%29 :type Float%20%28single-precision%29) (New%20Rotation%20Z%20%28Yaw%29 :type Float%20%28single-precision%29) (New%20Rotation%20X%20%28Roll%29 :type Float%20%28single-precision%29))
  (Transformation|SetWorldRotation (Variables|Default|GetMotionControllerLeft) (Math|Rotator|MakeRotator New%20Rotation%20X%20%28Roll%29 New%20Rotation%20Y%20%28Pitch%29 New%20Rotation%20Z%20%28Yaw%29) false false))

(event Custom|LeftLo
  (params (New%20Location%20Y :type Float%20%28double-precision%29) (New%20Location%20X :type Float%20%28double-precision%29) (New%20Location%20Z :type Float%20%28double-precision%29))
  (CallFunction|LeftControllerLoc New%20Location%20Y New%20Location%20X New%20Location%20Z))

(event Custom|LeftControllerLoc
  (params (New%20Location%20Y :type Float%20%28double-precision%29) (New%20Location%20X :type Float%20%28double-precision%29) (New%20Location%20Z :type Float%20%28double-precision%29))
  (Transformation|SetWorldLocation (Variables|Default|GetMotionControllerLeft) (Math|Vector|MakeVector New%20Location%20X New%20Location%20Y New%20Location%20Z) false false))

(event Custom|CamMoveM
  (params (New%20Location%20Y :type Float%20%28double-precision%29) (New%20Location%20X :type Float%20%28double-precision%29) (New%20Location%20Z :type Float%20%28double-precision%29))
  (Transformation|SetWorldLocation (Variables|Default|GetCamera) (Math|Vector|MakeVector New%20Location%20X New%20Location%20Y New%20Location%20Z) false false))

(event Custom|RightRo
  (params (New%20Rotation%20Y%20%28Pitch%29 :type Float%20%28single-precision%29) (New%20Rotation%20X%20%28Roll%29 :type Float%20%28single-precision%29) (New%20Rotation%20Z%20%28Yaw%29 :type Float%20%28single-precision%29))
  (CallFunction|RightControllerRot New%20Rotation%20Y%20%28Pitch%29 New%20Rotation%20Z%20%28Yaw%29 New%20Rotation%20X%20%28Roll%29))

(event Custom|Right%20ControllerRot
  (params (New%20Rotation%20Y%20%28Pitch%29 :type Float%20%28single-precision%29) (New%20Rotation%20Z%20%28Yaw%29 :type Float%20%28single-precision%29) (New%20Rotation%20X%20%28Roll%29 :type Float%20%28single-precision%29))
  (Transformation|SetWorldRotation (Variables|Default|GetMotionControllerRight) (Math|Rotator|MakeRotator New%20Rotation%20X%20%28Roll%29 New%20Rotation%20Y%20%28Pitch%29 New%20Rotation%20Z%20%28Yaw%29) false false))

(event Input|EnhancedActionEvents|EnhancedInputActionTriggers
  (params (ActionValue :type Float%20%28double-precision%29) (ElapsedSeconds :type Float%20%28double-precision%29) (TriggeredSeconds :type Float%20%28double-precision%29) (InputAction :type Input%20Action%20Object%20Reference :default "/Game/Blueprints/Widgets/Mappings/Triggers.Triggers"))
  (bind _widgetinteractionleft (Variables|Default|GetWidgetInteractionLeft))
  (:Started
    (Development|PrintString "LeftyLoosy")
    (Class|WidgetInteractionComponent|PressPointerKey _widgetinteractionleft "LeftMouseButton"))
  (:Completed
    (Class|WidgetInteractionComponent|ReleasePointerKey _widgetinteractionleft "LeftMouseButton")))

(event Input|EnhancedActionEvents|EnhancedInputActionTriggersRight
  (params (ActionValue :type Boolean) (ElapsedSeconds :type Float%20%28double-precision%29) (TriggeredSeconds :type Float%20%28double-precision%29) (InputAction :type Input%20Action%20Object%20Reference :default "/Game/Blueprints/Widgets/Mappings/TriggersRight.TriggersRight"))
  (bind _widgetinteractionright (Variables|Default|GetWidgetInteractionRight))
  (:Started
    (Development|PrintString "RightyTighty")
    (Class|WidgetInteractionComponent|PressPointerKey _widgetinteractionright "LeftMouseButton"))
  (:Completed
    (Class|WidgetInteractionComponent|ReleasePointerKey _widgetinteractionright "LeftMouseButton")))

(event EventBeginPlay
  (bind _asplayer_controller (Utilities|Casting|CastToPlayerController (Pawn|GetController)))
  (Utilities|IsValid (PlayerController|LocalPlayerSubsystems|GetEnhancedInputLocalPlayerSubsystem _asplayer_controller)
    (:Is%20Valid
      (Input|AddMappingContext (PlayerController|LocalPlayerSubsystems|GetEnhancedInputLocalPlayerSubsystem _asplayer_controller) "/Game/VRTemplate/Input/IMC_Trigger.IMC_Trigger" 0 "(bIgnoreAllPressedKeysUntilRelease=True,bForceImmediately=False)")
      (Networking|SetReplicates true)
      (Class|Actor|SetReplicateMovement true)
      (Input|AddMappingContext (PlayerController|LocalPlayerSubsystems|GetEnhancedInputLocalPlayerSubsystem _asplayer_controller) "/Game/Blueprints/Widgets/Mappings/TriggersMapping.TriggersMapping" 0 "(bIgnoreAllPressedKeysUntilRelease=True,bForceImmediately=False)"))))

(event EventTick
  (params (DeltaSeconds :type Float%20%28single-precision%29))
  (bind _camera (Variables|Default|GetCamera))
  (bind _camera_2 (Variables|Default|GetCamera))
  (bind _motioncontrollerright (Variables|Default|GetMotionControllerRight))
  (bind _motioncontrollerright_2 (Variables|Default|GetMotionControllerRight))
  (bind _motioncontrollerleft (Variables|Default|GetMotionControllerLeft))
  (bind _motioncontrollerleft_2 (Variables|Default|GetMotionControllerLeft))
  (bind _returnvalue (Transformation|GetWorldRotation _motioncontrollerleft))
  (bind _returnvalue_2 (Transformation|GetWorldLocation _motioncontrollerleft_2))
  (bind _returnvalue_3 (Transformation|GetWorldLocation _camera))
  (bind _returnvalue_4 (Transformation|GetWorldRotation _camera_2))
  (bind _returnvalue_5 (Transformation|GetWorldLocation _motioncontrollerright))
  (bind _returnvalue_6 (Transformation|GetWorldRotation _motioncontrollerright_2))
  (Utilities|FlowControl|Sequence
    (:then_0
      (CallFunction|WidgetInteractionPointer))
    (:then_1
      (Utilities|FlowControl|Delay 0.01)
      (CallFunction|CamMoveS (.y _returnvalue_3) (.x _returnvalue_3) (.z _returnvalue_3)))
    (:then_2
      (Utilities|FlowControl|Delay 0.01)
      (CallFunction|CamReplicateS (.pitch _returnvalue_4) (.roll _returnvalue_4) (.yaw _returnvalue_4)))
    (:then_3
      (Utilities|FlowControl|Delay 0.01)
      (CallFunction|RightLo (.y _returnvalue_5) (.x _returnvalue_5) (.z _returnvalue_5)))
    (:then_4
      (Utilities|FlowControl|Delay 0.01)
      (CallFunction|RightRo (.pitch _returnvalue_6) (.roll _returnvalue_6) (.yaw _returnvalue_6)))
    (:then_5
      (Utilities|FlowControl|Delay 0.01)
      (CallFunction|LeftLo (.y _returnvalue_2) (.x _returnvalue_2) (.z _returnvalue_2)))
    (:then_6
      (Utilities|FlowControl|Delay 0.01)
      (CallFunction|LeftRo (.pitch _returnvalue) (.roll _returnvalue) (.yaw _returnvalue)))))

(fn ConstructionScript)

(fn WidgetInteractionPointer
  (bind _widgetinteractionright (Variables|Default|GetWidgetInteractionRight))
  (bind _widgetinteractionleft (Variables|Default|GetWidgetInteractionLeft))
  (bind _returnvalue (Transformation|GetWorldLocation _widgetinteractionright))
  (bind _returnvalue_2 (Transformation|GetWorldLocation _widgetinteractionleft))
  (bind _returnvalue_3 (Class|WidgetInteractionComponent|GetLastHitResult _widgetinteractionleft))
  (bind _returnvalue_4 (Class|WidgetInteractionComponent|GetLastHitResult _widgetinteractionright))
  (bind _returnvalue_5 (Math|Rotator|FindLookatRotation _returnvalue_2 (.location _returnvalue_3)))
  (bind _returnvalue_6 (Math|Rotator|FindLookatRotation _returnvalue (.location _returnvalue_4)))
  (bind _returnvalue_7 (Math|Vector|GetForwardVector _returnvalue_5))
  (bind _returnvalue_8 (Math|Vector|GetForwardVector _returnvalue_6))
  (Utilities|FlowControl|Sequence
    (:then_0
      (bind _leftsplinemesh (Variables|Default|GetLeftSplineMesh)
        (:then
          (Components|DestroyComponent _leftsplinemesh))
        (:else
          _))
      (if (Class|WidgetInteractionComponent|IsOverHitTestVisibleWidget _widgetinteractionleft)
        (bind _returnvalue_9 (AddComponent|AddSplineMeshComponent true))
        (bind _output_get (Variables|Default|SetLeftSplineMesh _returnvalue_9))
        (SplineMesh|SetStartandEnd _output_get _returnvalue_2 _returnvalue_7 (.location _returnvalue_3) (* _returnvalue_7 (Math|Conversions|ToVector(Float) -1.0)) true :!class /Script/Engine.SplineMeshComponent)))
    (:then_1
      (bind _rightsplinemesh (Variables|Default|GetRightSplineMesh)
        (:then
          (Components|DestroyComponent _rightsplinemesh))
        (:else
          _))
      (if (Class|WidgetInteractionComponent|IsOverHitTestVisibleWidget _widgetinteractionright)
        (bind _returnvalue_10 (AddComponent|AddSplineMeshComponent true))
        (bind _output_get_2 (Variables|Default|SetRightSplineMesh _returnvalue_10))
        (SplineMesh|SetStartandEnd _output_get_2 _returnvalue _returnvalue_8 (.location _returnvalue_4) (* _returnvalue_8 (Math|Conversions|ToVector(Float) -1.0)) true :!class /Script/Engine.SplineMeshComponent)))))