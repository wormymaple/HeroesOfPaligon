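; Enemy laser beam actor aimed at the VR player's head hitbox with slight random Y/Z offset.
; BeginPlay grabs the first enemy and pawn found, then passes start and end points to the LaserBeam effect.
; A timeline drives Tick's lerp of a collision component from that enemy to the hit point, destroying the actor when finished.
; Overlapping a mesh component only sets the effect's IsColliding parameter.
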(event OnComponentBeginOverlap(Collision)
  (params (OverlappedComponent :type Primitive%20Component%20Object%20Reference) (OtherActor :type Actor%20Object%20Reference) (OtherComp :type Primitive%20Component%20Object%20Reference) (OtherBodyIndex :type Integer) (bFromSweep :type Boolean) (SweepResult :type Hit%20Result%20Structure%20%28by%20ref%29))
  (Utilities|Casting|CastToMeshComponent OtherComp)
  (Effects|Components|ParticleSystem|SetBoolParameter (Variables|Default|GetLaserBeam) "IsColliding" true))

(event Custom|LerpCollision
  (bind _lerp (Timeline|BeamLerp Play)
    (:Finished
      (Actor|DestroyActor))))

(event EventTick
  (params (DeltaSeconds :type Float%20%28single-precision%29))
  (Transformation|SetWorldLocation (Variables|Default|GetCollision) (Math|Vector|Lerp(Vector) (Transformation|GetActorLocation (Variables|Default|GetEnemyRef)) (Variables|Default|GetBeamHitPlayer) (stale Custom|LerpCollision _lerp)) false false))

(event EventBeginPlay
  (bind _returnvalue (Transformation|GetActorLocation))
  (bind _returnvalue_2 (Math|Random|RandomFloatinRange -1.0 1.0))
  (bind _returnvalue_3 (Math|Random|RandomFloatinRange -1.0 1.0))
  (bind _collision (Variables|Default|GetCollision))
  (bind _laserbeam (Variables|Default|GetLaserBeam))
  (Utilities|FlowControl|Sequence
    (:then_0
      (bind _outactors (Actor|GetAllActorsOfClass "/Game/VRTemplate/Blueprints/BP_BaseEnemy.BP_BaseEnemy_C"))
      (Variables|Default|SetEnemyRef (Utilities|Array|Get(acopy) _outactors))
      (bind _outactors_2 (Actor|GetAllActorsOfClass "/Game/VRTemplate/Blueprints/VRPawn.VRPawn_C"))
      (Variables|Default|SetPlayer%20Ref (Utilities|Array|Get(acopy) _outactors_2)))
    (:then_1
      (Effects|Components|ParticleSystem|SetVectorParameter _laserbeam "EnemyPosition" _returnvalue)
      (bind _output_get (Variables|Default|SetBeamHitPlayer (Math|Vector|MakeVector (.x (Transformation|GetWorldLocation (Variables|/Game/VRTemplate/Blueprints/VRPawn.VRPawn_C|GetHeadHitbox (Variables|Default|GetPlayer%20Ref)))) (+ (.y (Transformation|GetWorldLocation (Variables|/Game/VRTemplate/Blueprints/VRPawn.VRPawn_C|GetHeadHitbox (Variables|Default|GetPlayer%20Ref)))) _returnvalue_3) (+ (.z (Transformation|GetWorldLocation (Variables|/Game/VRTemplate/Blueprints/VRPawn.VRPawn_C|GetHeadHitbox (Variables|Default|GetPlayer%20Ref)))) _returnvalue_2))))
      (Variables|Default|SetAddedValue (Math|Vector|MakeVector 0.0 _returnvalue_3 _returnvalue_2))
      (Transformation|SetWorldLocation (Variables|Default|GetEndPoint) _output_get false false)
      (Effects|Components|ParticleSystem|SetVectorParameter _laserbeam "EndPoint" (Variables|Default|GetBeamHitPlayer)))
    (:then_2
      (CallFunction|LerpCollision))
    (:then_3
      (Transformation|SetWorldRotation _collision (Math|Rotator|FindLookatRotation (Transformation|GetWorldLocation _collision) (Transformation|GetWorldLocation (Variables|Default|GetEndPoint))) false false))
    (:then_4
      (Transformation|SetWorldLocation (Variables|Default|GetCollision) _returnvalue false false))))

(fn ConstructionScript)