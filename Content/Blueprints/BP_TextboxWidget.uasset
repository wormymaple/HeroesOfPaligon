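; BP_TextboxWidget is an actor that hosts a textbox widget and links it to an in-game keyboard.
; On BeginPlay it casts its Widget component's user widget to W_TextboxParent and binds to that widget's set-focus event.
; When focus is set, it passes itself to NewKeyboard, if valid, as the keyboard's focused widget.
; An unconnected duplicate of that update, using a Keyboard variable, never runs.
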(event Custom|NotifyKeyboard
  (Utilities|IsValid (Variables|Default|GetNewKeyboard)
    (:Is%20Valid
      (Default|UpdateFocusedWidget (Variables|Default|GetNewKeyboard) self))))

(event EventBeginPlay
  (bind _asw_textbox_parent (Utilities|Casting|CastToW_TextboxParent (UserInterface|GetUserWidgetObject (Variables|Default|GetWidget))))
  (EventDispatchers|BindEventtoOnSetFocus _asw_textbox_parent (delegate Custom|NotifyKeyboard)))

(event Collision|EventActorBeginOverlap
  (params (OtherActor :type Actor%20Object%20Reference)))

(event EventTick
  (params (DeltaSeconds :type Float%20%28single-precision%29)))

(fn ConstructionScript)