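; HOP_GI is the game instance that handles online lobby sessions and character customization saving.
; Lobby and private-match events create identical non-LAN sessions and open the Lobby as a listen server; joining and creation report failures through UI text.
; A separate event builds a random code, unused by sessions.
; Race changes trigger a HOP_Save write that zeroes every race, color and class field; color, class and load logic are unfinished.
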(event Custom|JoinSession
  (params (Session :type Blueprint%20Session%20Result%20Structure))
  ;[0.262 1 0.2266] Join Session
  (|JoinSession (Game|GetPlayerController 0) Session
    (:OnSuccess
      (Development|PrintString "Hello"))
    (:OnFailure
      (Default|Failed (Variables|Default|GetRering))
      (Variables|/Game/Blueprints/Widgets/Widgets/FailedCreateLobby.FailedCreateLobby_C|SetTextToDisplay (Variables|Default|GetNewVar) "Failed to Find A Lobby"))))

(event Custom|generate%20Code
  (Variables|Default|SetCode "")
  (for _index (range 0 4)
    (Variables|Default|SetCode (Utilities|String|Append (.OutItem (Utilities|Array|Random (Variables|Default|GetCharacterSet))) (Variables|Default|GetCode))))
  (Variables|Default|SetFinalCode (Variables|Default|GetCode))
  (Development|PrintString (Variables|Default|GetCode)))

(event Custom|Creating%20Private%20Match
  (params (NumberOfPlayers :type Integer))
  ;[1 0.05208 0.05208] Create Private Session
  (bind _output_get (Variables|Default|SetNumber%20Of%20Players NumberOfPlayers))
  (|Session (Game|GetPlayerController 0) _output_get false
    (:OnSuccess
      (Development|PrintString "Created?
")
      (Game|OpenLevel(byObjectReference) "/Game/Blueprints/Widgets/Levels/Lobby.Lobby" true "?listen"))
    (:OnFailure
      (Development|PrintString "Failed")
      (Default|Failed (Variables|Default|GetRering))
      (Variables|/Game/Blueprints/Widgets/Widgets/FailedCreateLobby.FailedCreateLobby_C|SetTextToDisplay (Variables|Default|GetNewVar) "Failed to Create A Lobby"))))

(event Custom|Changing%20Color
  ;[0.004949 1 0.9003] Change Color from Widget to actual actor its changing class to and saving it
)

(event Custom|CHangingCha
  ;[0.5588 0.237 1] Change Character from Widget to actual actor its changing class to and saving it
  (Default|ChangeRace (Variables|Default|Getnewbum))
  (CallFunction|SaveGame (Variables|Default|GetHOP%20SAVE%20SLOT)))

(event Custom|ChangeClass)

(event Custom|CreateLobbys
  (params (NumberOfPlayers :type Integer))
  ;[1 0.05208 0.05208] Create Session
  (bind _output_get (Variables|Default|SetNumber%20Of%20Players NumberOfPlayers))
  (|Session (Game|GetPlayerController 0) _output_get false
    (:OnSuccess
      (Development|PrintString "Created?
")
      (Game|OpenLevel(byObjectReference) "/Game/Blueprints/Widgets/Levels/Lobby.Lobby" true "?listen"))
    (:OnFailure
      (Development|PrintString "Failed")
      (Default|Failed (Variables|Default|GetRering))
      (Variables|/Game/Blueprints/Widgets/Widgets/FailedCreateLobby.FailedCreateLobby_C|SetTextToDisplay (Variables|Default|GetNewVar) "Failed to Create A Lobby"))))

(event EventInit)

(fn SaveGame
  (params (HOP_SAVE :type String))
  (bind _returnvalue (SaveGame|DoesSaveGameExist HOP_SAVE))
  (if _returnvalue
    (bind _returnvalue_2 (SaveGame|LoadGamefromSlot HOP_SAVE))
    (Variables|Default|SetHOP%20Save%20REF _returnvalue_2)
    (else
      (bind _returnvalue_3 (SaveGame|CreateSaveGameObject "/Game/Blueprints/HOP_Save.HOP_Save_C"))
      (bind _output_get (Variables|Default|SetHOP%20Save%20REF _returnvalue_3))))
  (bind _ashop_save (Utilities|Casting|CastToHOP_Save _output_get))
  (Variables|/Game/Blueprints/HOP_Save.HOP_Save_C|SetRace1 _ashop_save 0)
  (Variables|/Game/Blueprints/HOP_Save.HOP_Save_C|SetRace2 _ashop_save 0)
  (Variables|/Game/Blueprints/HOP_Save.HOP_Save_C|SetRace3 _ashop_save 0)
  (Variables|/Game/Blueprints/HOP_Save.HOP_Save_C|SetColor1 _ashop_save 0)
  (Variables|/Game/Blueprints/HOP_Save.HOP_Save_C|SetColor2 _ashop_save 0)
  (Variables|/Game/Blueprints/HOP_Save.HOP_Save_C|SetColor3 _ashop_save 0)
  (Variables|/Game/Blueprints/HOP_Save.HOP_Save_C|SetClass1 _ashop_save 0)
  (Variables|/Game/Blueprints/HOP_Save.HOP_Save_C|SetClass2 _ashop_save 0)
  (Variables|/Game/Blueprints/HOP_Save.HOP_Save_C|SetClass3 _ashop_save 0)
  (SaveGame|SaveGametoSlot (Variables|Default|GetHOP%20Save%20REF) HOP_SAVE)
  (Development|PrintString "Saed")
  (Development|PrintString (Utilities|String|ToString(Integer) 0))
  (Development|PrintString (Utilities|String|ToString(Integer) 0))
  (Development|PrintString (Utilities|String|ToString(Integer) 0)))

(fn LoadGame
  (params (HOP_SAVE :type String))
  (bind _returnvalue (SaveGame|DoesSaveGameExist HOP_SAVE))
  (if _returnvalue
    (bind _returnvalue_2 (SaveGame|LoadGamefromSlot HOP_SAVE))
    (bind _ashop_save (Utilities|Casting|CastToHOP_Save _returnvalue_2))))