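; VR keyboard actor whose widget component hosts W_Keyboard and binds it to a focused textbox widget.
; UpdateFocusedWidget stores the incoming textbox widget component, skipping the update when a valid one is already current.
; It casts that component's widget to W_TextboxParent, passes its root canvas panel to W_Keyboard as ParentCanvasPanel, then calls Start on the keyboard.
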(event Custom|UpdateFocusedWidget
  (params (Textbox%20Widget :type BP%20Textbox%20Widget%20Object%20Reference))
  (bind _widget (Variables|Default|GetWidget))
  (bind _returnvalue (UserInterface|GetUserWidgetObject _widget))
  (bind _asw_keyboard (Utilities|Casting|CastToW_Keyboard _returnvalue))
  (Utilities|IsValid Textbox%20Widget
    (:Is%20Valid
      (if (not (== (Variables|Default|GetCurrentTextboxWidget) Textbox%20Widget))
        (bind _output_get (Variables|Default|SetCurrentTextboxWidget Textbox%20Widget))
        (bind _asw_textbox_parent (Utilities|Casting|CastToW_TextboxParent (UserInterface|GetUserWidgetObject (Variables|/Game/Blueprints/BP_TextboxWidget.BP_TextboxWidget_C|GetWidget _output_get)) :!label _label))
        (Variables|/Game/AW_Widgets/W_KeyboardBase.W_KeyboardBase_C|SetParentCanvasPanel _asw_keyboard (Variables|/Game/AW_Widgets/W_TextboxParent.W_TextboxParent_C|GetCanvasPanel_0 _asw_textbox_parent))
        (Default|Start _asw_keyboard)))
    (:Is%20Not%20Valid
      (Variables|Default|SetCurrentTextboxWidget Textbox%20Widget)
      (goto _label))))

(event EventBeginPlay)

(event Collision|EventActorBeginOverlap
  (params (OtherActor :type Actor%20Object%20Reference)))

(event EventTick
  (params (DeltaSeconds :type Float%20%28single-precision%29)))

(fn ConstructionScript)