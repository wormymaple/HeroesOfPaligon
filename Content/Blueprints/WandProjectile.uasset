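; Wand projectile actor that damages enemies it overlaps and removes itself after a fixed lifetime.
; BeginPlay attaches an emitter and starts a delayed destroy.
; When the sphere overlaps a BP_BaseEnemy, it applies fixed damage, adds a Niagara effect, hides its visuals and disables sphere collision.
; The hit does not destroy the actor, which stays hidden until the timer expires; other actors are ignored.
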(event OnComponentBeginOverlap(Sphere)
  (params (OverlappedComponent :type Primitive%20Component%20Object%20Reference) (OtherActor :type Actor%20Object%20Reference) (OtherComp :type Primitive%20Component%20Object%20Reference) (OtherBodyIndex :type Integer) (bFromSweep :type Boolean) (SweepResult :type Hit%20Result%20Structure%20%28by%20ref%29))
  (bind _asbp_base_enemy (Utilities|Casting|CastToBP_BaseEnemy OtherActor))
  (Default|TakeDamage _asbp_base_enemy 4)
  (AddComponent|AddNiagaraComponent false)
  (Development|SetHiddeninGame (Variables|Default|GetSphere) true false)
  (Development|SetHiddeninGame (Variables|Default|GetSphere) true false)
  (Collision|SetCollisionEnabled (Variables|Default|GetSphere) "NoCollision"))

(event EventBeginPlay
  (Effects|SpawnEmitterAttached 0 0 "None")
  (Utilities|FlowControl|Delay 1e+01)
  (Actor|DestroyActor))

(event Collision|EventActorBeginOverlap
  (params (OtherActor :type Actor%20Object%20Reference)))

(event EventTick
  (params (DeltaSeconds :type Float%20%28single-precision%29)))

(fn ConstructionScript)