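; TestCharacter is a test Blueprint that previews race changes by swapping materials on a cube mesh.
; Its ChangeRace event switches over five temporary materials for Cube, but the selector is fixed at 0, so only the first is ever applied.
; Similar logic for Cube1 and Cube2 is disconnected, as is a cast to the HOP_GI game instance.
; BeginPlay, overlap and the construction script are empty.
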(event Custom|Change%20Race
  ;[0.2977 1 0.3244] Changing Race
  (switch int 0
    (:0
      (Rendering|Material|SetMaterial (Variables|Default|GetCube) 0 "/Game/Art/Materials/Temp1.Temp1"))
    (:1
      (Rendering|Material|SetMaterial (Variables|Default|GetCube) 0 "/Game/Art/Materials/Temp2.Temp2"))
    (:2
      (Rendering|Material|SetMaterial (Variables|Default|GetCube) 0 "/Game/Art/Materials/Temp3.Temp3"))
    (:3
      (Rendering|Material|SetMaterial (Variables|Default|GetCube) 0 "/Game/Art/Materials/Temp4.Temp4"))
    (:4
      (Rendering|Material|SetMaterial (Variables|Default|GetCube) 0 "/Game/Art/Materials/Temp5.Temp5"))))

(event EventBeginPlay)

(event Collision|EventActorBeginOverlap
  (params (OtherActor :type Actor%20Object%20Reference)))

(fn ConstructionScript)