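; BP_Sword is a melee weapon that damages BP_BaseEnemy actors overlapping its Cube2 component.
; Each accepted hit subtracts one point from EnemyHP and destroys the enemy at zero or below.
; Surviving enemies flash by briefly swapping the material on their head, chest, arms and legs.
; A DoOnce gate, reset after a delay, acts as a hit cooldown shared across all enemies.
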(event OnComponentBeginOverlap(Cube2)
  (params (OverlappedComponent :type Primitive%20Component%20Object%20Reference) (OtherActor :type Actor%20Object%20Reference) (OtherComp :type Primitive%20Component%20Object%20Reference) (OtherBodyIndex :type Integer) (bFromSweep :type Boolean) (SweepResult :type Hit%20Result%20Structure%20%28by%20ref%29))
  (bind _asbp_base_enemy (Utilities|Casting|CastToBP_BaseEnemy OtherActor))
  (Utilities|FlowControl|DoOnce false :!label _label
    (:Completed
      (bind _output_get (Variables|/Game/Blueprints/BP_BaseEnemy.BP_BaseEnemy_C|SetEnemyHP _asbp_base_enemy (- (Variables|/Game/Blueprints/BP_BaseEnemy.BP_BaseEnemy_C|GetEnemyHP _asbp_base_enemy) 1)))
      (if (<= _output_get 0)
        (Actor|DestroyActor _asbp_base_enemy)
        (else
          (Utilities|FlowControl|Sequence
            (:then_0
              (Rendering|Material|SetMaterial (Variables|/Game/Blueprints/BP_BaseEnemy.BP_BaseEnemy_C|GetChest _asbp_base_enemy) 0 "/Game/Blueprints/Widgets/Temp3.Temp3")
              (Utilities|FlowControl|Delay 0.2)
              (Rendering|Material|SetMaterial (Variables|/Game/Blueprints/BP_BaseEnemy.BP_BaseEnemy_C|GetChest _asbp_base_enemy) 0 "/Game/Blueprints/Widgets/Temp1.Temp1"))
            (:then_1
              (Rendering|Material|SetMaterial (Variables|/Game/Blueprints/BP_BaseEnemy.BP_BaseEnemy_C|GetLarm _asbp_base_enemy) 0 "/Game/Blueprints/Widgets/Temp3.Temp3")
              (Utilities|FlowControl|Delay 0.2)
              (Rendering|Material|SetMaterial (Variables|/Game/Blueprints/BP_BaseEnemy.BP_BaseEnemy_C|GetLarm _asbp_base_enemy) 0 "/Game/Blueprints/Widgets/Temp1.Temp1"))
            (:then_2
              (Rendering|Material|SetMaterial (Variables|/Game/Blueprints/BP_BaseEnemy.BP_BaseEnemy_C|GetRarm _asbp_base_enemy) 0 "/Game/Blueprints/Widgets/Temp3.Temp3")
              (Utilities|FlowControl|Delay 0.2)
              (Rendering|Material|SetMaterial (Variables|/Game/Blueprints/BP_BaseEnemy.BP_BaseEnemy_C|GetRarm _asbp_base_enemy) 0 "/Game/Blueprints/Widgets/Temp1.Temp1"))
            (:then_3
              (Rendering|Material|SetMaterial (Variables|/Game/Blueprints/BP_BaseEnemy.BP_BaseEnemy_C|GetLleg _asbp_base_enemy) 0 "/Game/Blueprints/Widgets/Temp3.Temp3")
              (Utilities|FlowControl|Delay 0.2)
              (Rendering|Material|SetMaterial (Variables|/Game/Blueprints/BP_BaseEnemy.BP_BaseEnemy_C|GetLleg _asbp_base_enemy) 0 "/Game/Blueprints/Widgets/Temp1.Temp1"))
            (:then_4
              (Rendering|Material|SetMaterial (Variables|/Game/Blueprints/BP_BaseEnemy.BP_BaseEnemy_C|GetRleg _asbp_base_enemy) 0 "/Game/Blueprints/Widgets/Temp3.Temp3")
              (Utilities|FlowControl|Delay 0.2)
              (Rendering|Material|SetMaterial (Variables|/Game/Blueprints/BP_BaseEnemy.BP_BaseEnemy_C|GetRleg _asbp_base_enemy) 0 "/Game/Blueprints/Widgets/Temp1.Temp1"))
            (:then_5
              (Rendering|Material|SetMaterial (Variables|/Game/Blueprints/BP_BaseEnemy.BP_BaseEnemy_C|GetHead _asbp_base_enemy) 0 "/Game/Blueprints/Widgets/Temp3.Temp3")
              (Utilities|FlowControl|Delay 0.2)
              (Rendering|Material|SetMaterial (Variables|/Game/Blueprints/BP_BaseEnemy.BP_BaseEnemy_C|GetHead _asbp_base_enemy) 0 "/Game/Blueprints/Widgets/Temp1.Temp1")))))
      (Utilities|FlowControl|Delay 1.0)
      (goto _label Reset))))

(fn ConstructionScript)