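; World-space lose-state widget actor that appears at BeginPlay only if the HOP_GI game instance's Lost flag is set.
; It destroys itself after five seconds, whether shown or hidden.
; Until then, FacePlayer re-triggers itself through a tiny Delay instead of using Tick, smoothly turning the actor's yaw toward the player controller's location.
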(event Custom|Face%20Player
  (Transformation|SetActorRotation (Math|Rotator|MakeRotator 0.0 0.0 (.yaw (Math|Interpolation|RInterpTo (Transformation|GetActorRotation) (Math|Rotator|FindLookatRotation (Transformation|GetActorLocation) (Transformation|GetActorLocation (Game|GetPlayerController 0))) (Utilities|Time|GetWorldDeltaSeconds) 2e+01))))
  (Utilities|FlowControl|Delay 0.001)
  (CallFunction|FacePlayer))

(event EventBeginPlay
  (Rendering|SetActorHiddenInGame true)
  (if (Variables|/Game/Blueprints/HOP_GI.HOP_GI_C|GetLost! (.AsHOP%20GI (Utilities|Casting|CastToHOP_GI (Game|GetGameInstance))))
    (Rendering|SetActorHiddenInGame false))
  (CallFunction|FacePlayer)
  (Utilities|FlowControl|Delay 5.0)
  (Actor|DestroyActor))

(event Collision|EventActorBeginOverlap
  (params (OtherActor :type Actor%20Object%20Reference)))

(event EventTick
  (params (DeltaSeconds :type Float%20%28single-precision%29)))

(fn ConstructionScript)