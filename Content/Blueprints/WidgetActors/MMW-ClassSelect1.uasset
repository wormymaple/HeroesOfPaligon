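; A class-select widget actor, judging by its name and folder, that keeps turning to face the first player.
; From BeginPlay, FacePlayer interpolates toward a look-at rotation aimed at the player controller's location and applies only the yaw.
; FacePlayer re-calls itself after a very short Delay, looping continuously in place of Tick, which is left empty.
; The graph contains no selection logic.
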(event Custom|Face%20Player
  (Transformation|SetActorRotation (Math|Rotator|MakeRotator 0.0 0.0 (.yaw (Math|Interpolation|RInterpTo (Transformation|GetActorRotation) (Math|Rotator|FindLookatRotation (Transformation|GetActorLocation) (Transformation|GetActorLocation (Game|GetPlayerController 0))) (Utilities|Time|GetWorldDeltaSeconds) 2e+01))))
  (Utilities|FlowControl|Delay 0.001)
  (CallFunction|FacePlayer))

(event EventBeginPlay
  (CallFunction|FacePlayer))

(event Collision|EventActorBeginOverlap
  (params (OtherActor :type Actor%20Object%20Reference)))

(event EventTick
  (params (DeltaSeconds :type Float%20%28single-precision%29)))

(fn ConstructionScript)