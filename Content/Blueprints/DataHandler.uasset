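; DataHandler is an actor that holds three player save-state slots for race, color, class and personality.
; BeginPlay seeds the struct array with three empty entries, and per-slot update events overwrite each index from its matching structure variable.
; Tick prints every slot's values each frame as a debug display.
; AddState appends CurrentStructure rather than its SaveState input, and UpdateSlot is an empty stub.
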(event Custom|UpdateSlot3
  (Utilities|Array|SetArrayElem (Variables|Default|GetPlayerInfoStructs) 2 (Variables|Default|GetSlot3Structure)))

(event Custom|UpdateSlot)

(event Custom|UpdateSlot1
  (Utilities|Array|SetArrayElem (Variables|Default|GetPlayerInfoStructs) 0 (Variables|Default|GetSlot1Structure)))

(event Custom|UpdateSlot2
  (Utilities|Array|SetArrayElem (Variables|Default|GetPlayerInfoStructs) 1 (Variables|Default|GetSlot2Structure)))

(event EventBeginPlay
  (bind _playersavestate (Utilities|Struct|MakePlayerSaveState))
  (bind _playerinfostructs (Variables|Default|GetPlayerInfoStructs))
  (Utilities|Array|Add _playerinfostructs _playersavestate)
  (Utilities|Array|Add _playerinfostructs _playersavestate)
  (Utilities|Array|Add _playerinfostructs _playersavestate))

(event Collision|EventActorBeginOverlap
  (params (OtherActor :type Actor%20Object%20Reference)))

(event EventTick
  (params (DeltaSeconds :type Float%20%28single-precision%29))
  (bind _playerinfostructs (Variables|Default|GetPlayerInfoStructs))
  (bind _playerinfostructs_2 (Variables|Default|GetPlayerInfoStructs))
  (bind _playerinfostructs_3 (Variables|Default|GetPlayerInfoStructs))
  (bind _output (Utilities|Array|Get(acopy) _playerinfostructs))
  (bind _output_2 (Utilities|Array|Get(acopy) _playerinfostructs_2 1))
  (bind _output_3 (Utilities|Array|Get(acopy) _playerinfostructs_3 2))
  (bind (_race _color _class _personality) (Utilities|Struct|BreakPlayerSaveState _output_3))
  (bind (_race_2 _color_2 _class_2 _personality_2) (Utilities|Struct|BreakPlayerSaveState _output))
  (bind (_race_3 _color_3 _class_3 _personality_3) (Utilities|Struct|BreakPlayerSaveState _output_2))
  (Development|PrintString (Utilities|String|ToString(Text) (Utilities|Text|FormatText "Slot 1 , Race {b}, Color {c}, Class {d}, Personality {e}" _race_2 _color_2 _class_2 _personality_2)) true true "(R=0.000000,G=0.660000,B=1.000000,A=1.000000)" DeltaSeconds)
  (Development|PrintString (Utilities|String|ToString(Text) (Utilities|Text|FormatText "Slot 2 , Race {b}, Color {c}, Class {d}, Personality {e}" _race_3 _color_3 _class_3 _personality_3)) true true "(R=0.000000,G=0.660000,B=1.000000,A=1.000000)" DeltaSeconds)
  (Development|PrintString (Utilities|String|ToString(Text) (Utilities|Text|FormatText "Slot 3 , Race {b}, Color {c}, Class {d}, Personality {e}" _race _color _class _personality)) true true "(R=0.000000,G=0.660000,B=1.000000,A=1.000000)" DeltaSeconds))

(fn ConstructionScript)

(fn AddState
  (params (SaveState :type Player%20Save%20State%20Structure))
  (Utilities|Array|Add (Variables|Default|GetPlayerInfoStructs) (Variables|Default|GetCurrentStructure)))